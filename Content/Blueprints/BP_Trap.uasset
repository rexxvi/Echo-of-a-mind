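; BP_Trap is a one-use trap actor that temporarily immobilises ghost enemies.
; When an overlapping actor tagged Ghost enters, it plays a scream, then sets the trapped flag on that BP_Enemy's BP_AIController and stops its movement.
; After an eight-second delay it clears the flag, sends the ghost to a random location in nav-walking mode and destroys itself.
; Player step-on sound and older trapping logic remain as unconnected nodes.
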(event EventBeginPlay)

(event EventTick
  (params (DeltaSeconds :type Float%20%28single-precision%29)))

(event Collision|EventActorBeginOverlap
  (params (OtherActor :type Actor%20Object%20Reference))
  (bind _output_get (Variables|Default|SetOther%20Actor OtherActor))
  (if (Actor|ActorHasTag _output_get "Ghost")
    (Audio|PlaySoundatLocation "/Game/Audio/SoundWaves/Effects/Ghost_scream.Ghost_scream" (Transformation|GetActorLocation (Variables|Default|GetOther%20Actor)) "0, 0, 0" 1.0 1.0 0.0 0 0 0 0)
    (bind _asbp_enemy (Utilities|Casting|CastToBP_Enemy (Variables|Default|GetOther%20Actor)))
    (bind _asbp_aicontroller (Utilities|Casting|CastToBP_AIController (AI|GetAIController _asbp_enemy)))
    (Default|SetIsTrapped _asbp_aicontroller true)
    (Components|Movement|StopMovementImmediately (Variables|/Script/Engine.Character|GetCharacterMovement _asbp_enemy))
    (Utilities|FlowControl|Delay 8.0)
    (Default|SetIsTrapped _asbp_aicontroller false)
    (Default|MovetoRandomLocation _asbp_aicontroller)
    (Pawn|Components|CharacterMovement|SetMovementMode (Variables|/Script/Engine.Character|GetCharacterMovement _asbp_enemy) "MOVE_NavWalking" 0)
    (Actor|DestroyActor)))

(fn ConstructionScript)