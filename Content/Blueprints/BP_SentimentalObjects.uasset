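; BP_SentimentalObjects is an interactable object that the player can use once while overlapping it.
; Overlap with a Player-tagged actor toggles IsInteractable and plays a sonar cue on entry.
; When interactable, Interact plays the supplied sound at the object, optionally tells BP_AIController to change movement to a given room, then destroys the object.
; Interact returns whether it succeeded; nothing in this graph actively calls it.
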(event EventBeginPlay)

(event Collision|EventActorBeginOverlap
  (params (OtherActor :type Actor%20Object%20Reference))
  (if (Actor|ActorHasTag OtherActor "Player")
    (Variables|Default|SetisInteractable true)
    (Audio|PlaySound2D "/Game/Audio/SoundCues/SC_sonarInteract.SC_sonarInteract" 1.0 1.0 0.0 0 0)))

(event EventTick
  (params (DeltaSeconds :type Float%20%28single-precision%29)))

(event Collision|EventActorEndOverlap
  (params (OtherActor :type Actor%20Object%20Reference))
  (if (Actor|ActorHasTag OtherActor "Player")
    (Variables|Default|SetisInteractable false)))

(fn ConstructionScript)

(fn Interact
  (params (SoundToPlay :type Sound%20Base%20Object%20Reference) (SwitchToRoom :type Boolean) (RoomNumber :type Integer))
  (if (Variables|Default|GetisInteractable)
    (Audio|PlaySoundatLocation SoundToPlay (Transformation|GetActorLocation) "0, 0, 0" 1.0 1.0 0.0 0 0 0 0)
    (if SwitchToRoom
      (bind _returnvalue (Actor|GetActorOfClass "/Game/Blueprints/BP_AIController.BP_AIController_C"))
      (Default|ChangeMovement _returnvalue RoomNumber)
      (Development|PrintString (Utilities|String|Append "Changing to Room: " (Utilities|String|ToString(Integer) RoomNumber))))
    (Actor|DestroyActor)
    (return true)
    (else
      (return false))))