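; BP_Ghost is a ghost hazard that sends the player back to a fixed point on contact.
; On overlap with the player pawn, it plays an attack sound, teleports the pawn to a hard-coded location and zeroes the control rotation.
; BeginPlay calls MoveToRandomLocation, but that event is empty.
; The looping random navmesh wander via AIMoveTo is disconnected and never runs.
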(event Custom|Move%20to%20random%20location)

(event Collision|EventActorBeginOverlap
  (params (OtherActor :type Actor%20Object%20Reference))
  (if (== OtherActor (Game|Player|GetPlayerPawn 0))
    (Audio|PlaySoundatLocation "/Game/Audio/SoundCues/SC_GhostAttack.SC_GhostAttack" (Transformation|GetActorLocation) "0, 0, 0" 1.0 1.0 0.0 0 0 0 0)
    (Transformation|SetActorLocation (Game|Player|GetPlayerPawn 0) "2850.000000,-90.000000,100.000000" false false)
    (Pawn|SetControlRotation (Game|GetPlayerController 0) (Math|Rotator|MakeRotator 0.0 0.0 0.0))))

(event EventBeginPlay
  (CallFunction|MovetoRandomLocation))

(fn ConstructionScript)